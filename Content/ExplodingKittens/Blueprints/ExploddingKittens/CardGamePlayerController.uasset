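; CardGamePlayerController is the player controller for an Exploding Kittens card game.
; Every tick it casts the game state to CardGameGameState and calls UpdateSelectionObjects on the main and discard decks.
; It then casts the first player pawn to CardGamePawn but does nothing with it, leaving the hand-card count lookup unconnected.
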(event EventBeginPlay)

(event EventTick
  (params (DeltaSeconds :type Float%20%28single-precision%29))
  (bind _ascard_game_game_state (Utilities|Casting|CastToCardGameGameState (Game|GetGameState)))
  (Default|UpdateSelectionObjects (Variables|/Game/ExplodingKittens/Blueprints/ExploddingKittens/CardGameGameState.CardGameGameState_C|GetMainDeck _ascard_game_game_state))
  (Default|UpdateSelectionObjects (Variables|/Game/ExplodingKittens/Blueprints/ExploddingKittens/CardGameGameState.CardGameGameState_C|GetDiscardDeck _ascard_game_game_state))
  (bind _ascard_game_pawn (Utilities|Casting|CastToCardGamePawn (Game|Player|GetPlayerPawn 0))))

(fn ConstructionScript)