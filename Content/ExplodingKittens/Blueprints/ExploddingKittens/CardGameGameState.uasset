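; Game state for the Exploding Kittens card game that tracks whose turn it is and holds references to the decks.
; On BeginPlay it gathers all card game pawns, possesses the first, and finds the discard and main decks by actor tag.
; AdvanceTurnPlayer wraps the turn index around the player count and moves player controller 0 onto that player's pawn, so one controller serves every player in turn.
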(event EventBeginPlay
  (Utilities|FlowControl|Sequence
    (:then_0
      (bind _outactors (Actor|GetAllActorsOfClass "/Game/ExplodingKittens/Blueprints/ExploddingKittens/CardGamePawn.CardGamePawn_C"))
      (bind _output_get (Variables|Default|SetPlayerPawns _outactors))
      (Pawn|Possess (Game|GetPlayerController 0) (Utilities|Array|Get(acopy) _output_get)))
    (:then_1
      (bind _outactors_2 (Actor|GetAllActorsOfClasswithTag "/Game/ExplodingKittens/Blueprints/ExploddingKittens/Deck.Deck_C" "Discard"))
      (bind _asdeck (Utilities|Casting|CastToDeck (Utilities|Array|Get(acopy) _outactors_2)))
      (Variables|Default|SetDiscardDeck _asdeck))
    (:then_2
      (bind _outactors_3 (Actor|GetAllActorsOfClasswithTag "/Game/ExplodingKittens/Blueprints/ExploddingKittens/Deck.Deck_C" "MainDeck"))
      (bind _asdeck_2 (Utilities|Casting|CastToDeck (Utilities|Array|Get(acopy) _outactors_3)))
      (Variables|Default|SetMainDeck _asdeck_2))))

(fn ConstructionScript)

(fn AdvanceTurnPlayer
  (Variables|Default|SetTurnPlayer (select (== (+ (Variables|Default|GetTurnPlayer) 1) (Variables|Default|GetNumPlayers)) 0 (+ (Variables|Default|GetTurnPlayer) 1)))
  (Pawn|UnPossess (Game|GetPlayerController 0))
  (Pawn|Possess (Game|GetPlayerController 0) (Utilities|Array|Get(acopy) (Variables|Default|GetPlayerPawns) (Variables|Default|GetTurnPlayer))))