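; CardGameHUD is the HUD for the Exploding Kittens card game, creating all of its UI widgets up front on BeginPlay.
; A Sequence creates each widget, stores it in a variable and adds it to the viewport.
; The main and start screens stay visible, while the input, Nope, player and card choice, scry, combo and end-game screens begin hidden.
; It holds no logic to show them again.
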(event EventBeginPlay
  (Utilities|FlowControl|Sequence
    (:then_0
      ;[1 1 1] Set the input mode to UI only
      (bind _returnvalue (UserInterface|CreateWidget "/Game/ExplodingKittens/Blueprints/ExploddingKittens/MainUI.MainUI_C"))
      (bind _output_get (Variables|Default|SetMainUI _returnvalue))
      (UserInterface|Viewport|AddtoViewport _output_get 0))
    (:then_1
      (bind _returnvalue_2 (UserInterface|CreateWidget "/Game/ExplodingKittens/Blueprints/ExploddingKittens/StartUI.StartUI_C"))
      (bind _output_get_2 (Variables|Default|SetStartUI _returnvalue_2))
      (UserInterface|Viewport|AddtoViewport _output_get_2 0))
    (:then_2
      (bind _returnvalue_3 (UserInterface|CreateWidget "/Game/ExplodingKittens/Blueprints/ExploddingKittens/InputUI.InputUI_C"))
      (bind _output_get_3 (Variables|Default|SetInputUI _returnvalue_3))
      (UserInterface|Viewport|AddtoViewport _output_get_3 0)
      (Widget|SetVisibility _output_get_3 "Hidden"))
    (:then_3
      (bind _returnvalue_4 (UserInterface|CreateWidget "/Game/ExplodingKittens/Blueprints/ExploddingKittens/NopeUI.NopeUI_C"))
      (bind _output_get_4 (Variables|Default|SetNopeUI _returnvalue_4))
      (UserInterface|Viewport|AddtoViewport _output_get_4 0)
      (Widget|SetVisibility _output_get_4 "Hidden"))
    (:then_4
      (bind _returnvalue_5 (UserInterface|CreateWidget "/Game/ExplodingKittens/Blueprints/ExploddingKittens/NopeUI_2.NopeUI_2_C"))
      (bind _output_get_5 (Variables|Default|SetChoosePLayerUI _returnvalue_5))
      (UserInterface|Viewport|AddtoViewport _output_get_5 0)
      (Widget|SetVisibility _output_get_5 "Hidden"))
    (:then_5
      (bind _returnvalue_6 (UserInterface|CreateWidget "/Game/ExplodingKittens/Blueprints/ExploddingKittens/InputUI_2.InputUI_2_C"))
      (bind _output_get_6 (Variables|Default|SetChooseCardUI _returnvalue_6))
      (UserInterface|Viewport|AddtoViewport _output_get_6 0)
      (Widget|SetVisibility _output_get_6 "Hidden"))
    (:then_6
      (bind _returnvalue_7 (UserInterface|CreateWidget "/Game/ExplodingKittens/Blueprints/ExploddingKittens/ScryUI.ScryUI_C"))
      (bind _output_get_7 (Variables|Default|SetScryUI _returnvalue_7))
      (UserInterface|Viewport|AddtoViewport _output_get_7 0)
      (Widget|SetVisibility _output_get_7 "Hidden"))
    (:then_7
      (bind _returnvalue_8 (UserInterface|CreateWidget "/Game/ExplodingKittens/Blueprints/ExploddingKittens/ENDGAMEUI.ENDGAMEUI_C"))
      (bind _output_get_8 (Variables|Default|SetEndGameUI _returnvalue_8))
      (UserInterface|Viewport|AddtoViewport _output_get_8 0)
      (Widget|SetVisibility _output_get_8 "Hidden"))
    (:then_8
      (bind _returnvalue_9 (UserInterface|CreateWidget "/Game/ExplodingKittens/Blueprints/ExploddingKittens/NopeUI_3.NopeUI_3_C"))
      (bind _output_get_9 (Variables|Default|SetChooseComboPlayerUI _returnvalue_9))
      (UserInterface|Viewport|AddtoViewport _output_get_9 0)
      (Widget|SetVisibility _output_get_9 "Hidden"))
    (:then_9
      (bind _returnvalue_10 (UserInterface|CreateWidget "/Game/ExplodingKittens/Blueprints/ExploddingKittens/ComboUI.ComboUI_C"))
      (bind _output_get_10 (Variables|Default|SetComboUI _returnvalue_10))
      (UserInterface|Viewport|AddtoViewport _output_get_10 0)
      (Widget|SetVisibility _output_get_10 "Hidden"))))

(fn ConstructionScript)